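; BP_Jump_Powerup is a jump power-up pickup with a static mesh whose yaw is animated by the RotateBoot timeline from BeginPlay.
; A box overlap with any actor whose display name contains "Third" plays a pitched-up sound.
; It then casts player 0's character, rather than the overlapping actor, to ThirdPersonCharacter, calls JumpPowerUp on it and destroys the pickup.
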(event `self.ReceiveBeginPlay`
  (bind (_direction _newtrack_0) (`Timeline|Rotate Boot` :!via `PlayFromStart`)
    (:`Update`
      (`SceneComponent.K2_SetRelativeRotation` (`self.StaticMesh`) (`KismetMathLibrary.MakeRotator` 0.0 0.0 _newtrack_0) false false))))

(event `self.Box.OnComponentBeginOverlap`
  (params (OverlappedComponent :type "PrimitiveComponent Object Reference") (OtherActor :type "Actor Object Reference") (OtherComp :type "PrimitiveComponent Object Reference") (OtherBodyIndex :type Integer) (bFromSweep :type Boolean) (SweepResult :type "HitResult Structure (by ref)"))
  (if (`KismetStringLibrary.Contains` (`KismetSystemLibrary.GetDisplayName` OtherActor) "Third")
    (`GameplayStatics.PlaySound2D` "/Game/MyContent/Sounds/power_up.power_up" 0.33 2.0 3.2 null null)
    (bind _asthird_person_character (cast `/Game/MyContent/Blueprints/ThirdPersonCharacter/ThirdPersonCharacter` (`GameplayStatics.GetPlayerCharacter` 0)))
    (`/Game/MyContent/Blueprints/ThirdPersonCharacter/ThirdPersonCharacter.JumpPowerUp` _asthird_person_character)
    (`self.K2_DestroyActor`)))

(fn `UserConstructionScript`)