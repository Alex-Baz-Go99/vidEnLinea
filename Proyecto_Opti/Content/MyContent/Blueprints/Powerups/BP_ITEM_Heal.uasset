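; BP_ITEM_Heal is a heal item pickup that goes into the inventory of the actor touching it.
; Its Box overlap identifies the collector by checking for "Third" in the actor's display name, then plays a pitched-up Power_up sound.
; It passes one unit of its ObjectStructure to that actor's COM_Inventory via AddObject.
; The pickup destroys itself only if the add succeeds, though the sound plays either way.
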(event `self.Box.OnComponentBeginOverlap`
  (params (OverlappedComponent :type "PrimitiveComponent Object Reference") (OtherActor :type "Actor Object Reference") (OtherComp :type "PrimitiveComponent Object Reference") (OtherBodyIndex :type Integer) (bFromSweep :type Boolean) (SweepResult :type "HitResult Structure (by ref)"))
  (if (`KismetStringLibrary.Contains` (`KismetSystemLibrary.GetDisplayName` OtherActor) "Third")
    (`GameplayStatics.PlaySound2D` "/Game/MyContent/Sounds/power_up.power_up" 0.33 2.0 3.2 null null)
    (bind _wasadded_ (`/Game/MyContent/Blueprints/Inventory/COM_Inventory.AddObject` (`self.GetComponentByClass` OtherActor "/Game/MyContent/Blueprints/Inventory/COM_Inventory.COM_Inventory_C") (make `/Game/MyContent/Blueprints/Inventory/EST_Space` (`self.ObjectStructure`) 1)))
    (if _wasadded_
      (`self.K2_DestroyActor`))))

(fn `UserConstructionScript`
  (`parent.UserConstructionScript`))