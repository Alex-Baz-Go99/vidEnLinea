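; BP_Super_Lasergun is a laser gun that fires a BP_Bullet_2 projectile with a three-second cooldown.
; ClientFire2 and ServerFire2 store the Parent reference and share one firing path gated by a boolean.
; That path plays the shot sound, spawns the bullet at the skeletal mesh's "so" socket and passes Parent to it.
; After the delay, a ready sound plays and the gate reopens.
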(event `Client Fire2`
  (params (Parent :type "/Game/MyContent/Blueprints/ThirdPersonCharacter/ThirdPersonCharacter Object Reference"))
  (set `self.Parent` Parent)
  (if (`self.bool`) :!label _label
    (`GameplayStatics.SpawnSoundAtLocation` "/Game/MyContent/Sounds/Disparos.Disparos" (`SceneComponent.K2_GetComponentLocation` (`self.SkeletalMesh`)) (struct) 1.0 0.66 0.0 null null)
    (bind _returnvalue (`|SpawnActorFromClass` "/Game/MyContent/Blueprints/Guns/BP_Bullet_2.BP_Bullet_2_C" (`SceneComponent.GetSocketTransform` (`self.SkeletalMesh`) "so" "RTS_World") "AlwaysSpawn" "OverrideRootScale" null null))
    (set `/Game/MyContent/Blueprints/Guns/BP_Bullet_2.Parent` (`self.Parent`) _returnvalue)
    (set `self.bool` false)
    (`KismetSystemLibrary.Delay` 3.0)
    (`GameplayStatics.SpawnSoundAtLocation` "/Game/MyContent/Sounds/GunReady.GunReady" (`SceneComponent.K2_GetComponentLocation` (`self.SkeletalMesh`)) (struct) 0.15 0.66 0.0 null null)
    (set `self.bool` true)))

(event `Server Fire2`
  (params (Parent :type "/Game/MyContent/Blueprints/ThirdPersonCharacter/ThirdPersonCharacter Object Reference"))
  (set `self.Parent` Parent)
  (goto _label))

(fn `UserConstructionScript`)