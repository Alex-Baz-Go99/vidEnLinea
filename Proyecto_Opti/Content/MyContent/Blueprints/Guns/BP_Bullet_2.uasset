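; Bullet projectile that moves itself each tick along a velocity set from its forward vector, scaled by half the squared frame time.
; A line trace between previous and next positions detects hits, identifying targets by name substring.
; ThirdPersonCharacters other than Parent take fixed damage and destroy the bullet, which otherwise expires after a short delay.
; Hits on "Des" actors spawn a BP_MassObject, push it with the bullet's velocity, then immediately destroy it.
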(event `self.ReceiveTick`
  (params (DeltaSeconds :type "Float (single-precision)"))
  (`|ExecutionSequence`
    (:`then_0`
      (set `self.prevPosition` (`self.K2_GetActorLocation`))
      (bind _output_get (set `self.nextPosition` (+ (* (* (`self.velocity`) (`KismetMathLibrary.MultiplyMultiply_FloatFloat` DeltaSeconds 2.0)) 0.5) (`self.K2_GetActorLocation`))))
      (`self.K2_SetActorLocation` _output_get)
      (bind (_damage _player) (`self.DetectHit`))
      (if _damage
        (message `/Game/MyContent/Blueprints/Interfaces/BPI_Damageable.Take Damage` _player 50.0)
        (`self.K2_DestroyActor` :!label _label)))
    (:`then_1`
      (`KismetSystemLibrary.Delay` 2.0)
      (goto _label))))

(event `self.ReceiveBeginPlay`
  (set `self.velocity` (* (`self.GetActorForwardVector`) (`self.initial speed`))))

(fn `DetectHit`
  (returns (Damage :type Boolean) (Player :type "/Game/MyContent/Blueprints/ThirdPersonCharacter/ThirdPersonCharacter Object Reference") (HitActor :type "Actor Object Reference"))
  (bind (_outhit _returnvalue) (`KismetSystemLibrary.LineTraceSingle` (`self.prevPosition`) (`self.nextPosition`) "TraceTypeQuery2"))
  (if _returnvalue
    (bind (_bblockinghit _binitialoverlap _time _distance _location _impactpoint _normal _impactnormal _physmat _hitactor) (`GameplayStatics.BreakHitResult` _outhit))
    (bind _returnvalue_2 (`KismetSystemLibrary.GetObjectName` _hitactor))
    (if (`KismetStringLibrary.Contains` _returnvalue_2 "Third")
      (if (not (== _hitactor (`self.Parent`)))
        (bind _asthird_person_character (cast `/Game/MyContent/Blueprints/ThirdPersonCharacter/ThirdPersonCharacter` _hitactor))
        (return true _asthird_person_character _asthird_person_character))
      (elif (`KismetStringLibrary.Contains` _returnvalue_2 "Des")
        (bind _returnvalue_3 (`|SpawnActorFromClass` "/Game/MyContent/Blueprints/Guns/BP_MassObject.BP_MassObject_C" (`self.GetTransform`) "Undefined" "OverrideRootScale" null null))
        (`PrimitiveComponent.AddForce` (`/Game/MyContent/Blueprints/Guns/BP_MassObject.Sphere` _returnvalue_3) (`self.velocity`) "None" false)
        (`self.K2_DestroyActor` _returnvalue_3)
        (return false null null)))))

(fn `UserConstructionScript`)