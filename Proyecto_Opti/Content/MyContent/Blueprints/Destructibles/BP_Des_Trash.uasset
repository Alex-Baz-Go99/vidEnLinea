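; BP_Des_Trash is a destructible trash prop that explodes when shot.
; On BeginPlay, a timeline moves StaticMesh vertically by adding its track value to the current relative Z each update.
; A box overlap with an actor named "Bullet" without a "2" teleports StaticMesh1 below and reveals the Destructible in its place.
; It then spawns explosion particles, plays a 2D sound and destroys the actor after a short delay.
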(event `self.ReceiveBeginPlay`
  (bind _staticmesh (`self.StaticMesh`))
  (bind (_direction _newtrack_0) (`Timeline|Timeline_0`)
    (:`Update`
      (`SceneComponent.K2_SetRelativeLocation` _staticmesh (+ (`KismetMathLibrary.MakeVector` 0.0 0.0 _newtrack_0) (`SceneComponent.RelativeLocation` _staticmesh)) false false))))

(event `self.Box.OnComponentBeginOverlap`
  (params (OverlappedComponent :type "PrimitiveComponent Object Reference") (OtherActor :type "Actor Object Reference") (OtherComp :type "PrimitiveComponent Object Reference") (OtherBodyIndex :type Integer) (bFromSweep :type Boolean) (SweepResult :type "HitResult Structure (by ref)"))
  (bind _returnvalue (`KismetSystemLibrary.GetObjectName` OtherActor))
  (bind _destructible (`self.Destructible`))
  (if (`KismetStringLibrary.Contains` _returnvalue "Bullet")
    (if (not (`KismetStringLibrary.Contains` _returnvalue "2"))
      (`SceneComponent.K2_SetRelativeLocation` (`self.StaticMesh1`) (0.0 0.0 -1000.0) false true)
      (`SceneComponent.SetVisibility` _destructible true false)
      (`SceneComponent.K2_SetRelativeLocation` _destructible (0.0 0.0 0.0) false true)
      (`GameplayStatics.SpawnEmitterAtLocation` "/Game/MyContent/Particulas/Explosion_Particles.Explosion_Particles" (`SceneComponent.K2_GetComponentLocation` (`self.Box`)))
      (`GameplayStatics.PlaySound2D` "/Game/MyContent/Sounds/Explosion.Explosion" 0.2 1.0 0.0 null null)
      (`KismetSystemLibrary.Delay` 1.0)
      (`self.K2_DestroyActor`))))

(fn `UserConstructionScript`)