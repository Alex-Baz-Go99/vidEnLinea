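; Streetlamp actor with two spotlights that switch on and off on a timeline schedule and cast shadows only near the player.
; A timeline started at BeginPlay sets both lights to full intensity while its track value falls within either of two ranges, and to zero otherwise.
; Box overlap events toggle shadow casting on both lights, identifying the player by a "ThirdPersonCharacter" substring in the actor's name.
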(event `self.ReceiveBeginPlay`
  (bind _spotlight (`self.SpotLight`))
  (bind _spotlight1 (`self.SpotLight1`))
  (bind (_direction _newtrack_0) (`Timeline|Timeline_0` :!via `PlayFromStart`)
    (:`Update`
      (if (or (`KismetMathLibrary.InRange_FloatFloat` _newtrack_0 180.0 192.0) (`KismetMathLibrary.InRange_FloatFloat` _newtrack_0 370.0 540.0))
        (`|ExecutionSequence`
          (:`then_0`
            (`LightComponent.SetIntensity` _spotlight 80000.0))
          (:`then_1`
            (`LightComponent.SetIntensity` _spotlight1 80000.0)))
        (else
          (`|ExecutionSequence`
            (:`then_0`
              (`LightComponent.SetIntensity` _spotlight 0.0))
            (:`then_1`
              (`LightComponent.SetIntensity` _spotlight1 0.0))))))))

(event `self.ReceiveTick`
  (params (DeltaSeconds :type "Float (single-precision)")))

(event `self.Box.OnComponentBeginOverlap`
  (params (OverlappedComponent :type "PrimitiveComponent Object Reference") (OtherActor :type "Actor Object Reference") (OtherComp :type "PrimitiveComponent Object Reference") (OtherBodyIndex :type Integer) (bFromSweep :type Boolean) (SweepResult :type "HitResult Structure (by ref)"))
  (if (`KismetStringLibrary.Contains` (`KismetSystemLibrary.GetObjectName` OtherActor) "ThirdPersonCharacter")
    (`|ExecutionSequence`
      (:`then_0`
        (`LightComponentBase.SetCastShadows` (`self.SpotLight`) true))
      (:`then_1`
        (`LightComponentBase.SetCastShadows` (`self.SpotLight1`) true)))))

(event `self.Box.OnComponentEndOverlap`
  (params (OverlappedComponent :type "PrimitiveComponent Object Reference") (OtherActor :type "Actor Object Reference") (OtherComp :type "PrimitiveComponent Object Reference") (OtherBodyIndex :type Integer))
  (if (`KismetStringLibrary.Contains` (`KismetSystemLibrary.GetObjectName` OtherActor) "ThirdPersonCharacter")
    (`|ExecutionSequence`
      (:`then_0`
        (`LightComponentBase.SetCastShadows` (`self.SpotLight`) false))
      (:`then_1`
        (`LightComponentBase.SetCastShadows` (`self.SpotLight1`) false)))))

(fn `UserConstructionScript`)