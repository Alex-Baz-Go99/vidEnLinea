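; Inventory component that holds items in a fixed-size slot array and toggles the inventory widget on screen.
; AddObject tops up a non-full stack of the same Type, recursing with any overflow, otherwise fills the first empty slot.
; It always returns true, with no check for a full inventory.
; OpenClose creates or removes WB_Inventory on the ThirdPersonCharacter's HUD canvas, switching cursor and input mode.
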(event `self.ReceiveBeginPlay`
  (`self.InitInventory`))

(fn `AddObject`
  (params (AddContent :type "/Game/MyContent/Blueprints/Inventory/EST_Space Structure"))
  (returns (`WasAdded?` :type Boolean))
  (bind _addcontent (`local.AddContent`))
  (if (`.IsStackable?_10_6F1F98664534A4753AD90D830CB20E17` (break `/Game/MyContent/Blueprints/Inventory/EST_Object` (break `/Game/MyContent/Blueprints/Inventory/EST_Space` AddContent)))
    (bind _indexstack (`self.StackMacro` _addcontent)
      (:`True`
        (`self.AddStack` (`local.AddContent`) _indexstack))
      (:`False`
        (`self.CreateStack` _addcontent :!label _label)))
    (else
      (goto _label)))
  (return true))

(fn `AddStack`
  (params (SpaceStructure :type "/Game/MyContent/Blueprints/Inventory/EST_Space Structure") (SpaceIndex :type Integer))
  (bind _inventory (`self.Inventory`))
  (bind _spaceindex (`local.SpaceIndex`))
  (bind (_spacestructure_objectstructure _spacestructure_amount) (break `/Game/MyContent/Blueprints/Inventory/EST_Space` (`local.SpaceStructure`)))
  (bind _spacestructure_objectstructure_2 (break `/Game/MyContent/Blueprints/Inventory/EST_Space` (`local.SpaceStructure`)))
  (bind (_spacestructure_objectstructure_3 _spacestructure_amount_2) (break `/Game/MyContent/Blueprints/Inventory/EST_Space` (`local.SpaceStructure`)))
  (bind (_name _isstackable_ _image _maxstackable) (break `/Game/MyContent/Blueprints/Inventory/EST_Object` _spacestructure_objectstructure_2))
  (bind _output (`|GetArrayItem` (`self.Inventory`) SpaceIndex))
  (bind (_output_objectstructure _output_amount) (break `/Game/MyContent/Blueprints/Inventory/EST_Space` (`|GetArrayItem` _inventory _spaceindex)))
  (bind _output_get (set `self.CurrentAmount` (`.Amount_5_90D960ED4D5A51A72869D1BC7F1CD284` (break `/Game/MyContent/Blueprints/Inventory/EST_Space` _output))))
  (if (> (+ (`.Amount_5_90D960ED4D5A51A72869D1BC7F1CD284` (break `/Game/MyContent/Blueprints/Inventory/EST_Space` SpaceStructure)) _output_get) (`.MaxStackable_13_6927FB4A4C4F7AAE766A8C8979463C00` (break `/Game/MyContent/Blueprints/Inventory/EST_Object` (break `/Game/MyContent/Blueprints/Inventory/EST_Space` _output))))
    (`KismetArrayLibrary.Array_Set` (`self.Inventory`) (`local.SpaceIndex`) (make `/Game/MyContent/Blueprints/Inventory/EST_Space` _spacestructure_objectstructure_2 _maxstackable))
    (`self.AddObject` (make `/Game/MyContent/Blueprints/Inventory/EST_Space` _spacestructure_objectstructure_3 (- _spacestructure_amount_2 (- _maxstackable (`self.CurrentAmount`)))))
    (else
      (`KismetArrayLibrary.Array_Set` _inventory _spaceindex (make `/Game/MyContent/Blueprints/Inventory/EST_Space` _output_objectstructure (+ _spacestructure_amount _output_amount)))))
  (return))

(fn `CreateStack`
  (params (AddContent :type "/Game/MyContent/Blueprints/Inventory/EST_Space Structure"))
  (bind _inventory (`self.Inventory`))
  (`KismetArrayLibrary.Array_Set` _inventory (`KismetArrayLibrary.Array_Find` _inventory (make `/Game/MyContent/Blueprints/Inventory/EST_Space` (struct :`Name` "NSLOCTEXT(\"[8A8A146A4B9932E402FF018AC5B0D078]\", \"E9B93D44448122FA83936192D0E27268\", \"None\")" :`IsStackable?` true))) AddContent))

(fn `InitInventory`
  (`KismetArrayLibrary.Array_Resize` (`self.Inventory`) (`self.Space`)))

(fn `OpenClose`
  (bind _returnvalue (`GameplayStatics.GetPlayerController` 0))
  (bind _returnvalue_2 (`GameplayStatics.GetPlayerController` 0))
  (bind _inventorywidget (`self.InventoryWidget`))
  (bind _inventorywidget_2 (`self.InventoryWidget`)
    (:`then`
      (`Widget.RemoveFromParent` _inventorywidget_2)
      (set `self.InventoryWidget` null)
      (set `PlayerController.bShowMouseCursor` false _returnvalue)
      (`WidgetBlueprintLibrary.SetInputMode_GameOnly` _returnvalue))
    (:`else`
      (bind _returnvalue_3 (`|CreateWidget` "/Game/MyContent/Blueprints/Inventory/Widgets/WB_Inventory.WB_Inventory_C" (`GameplayStatics.GetPlayerController` 0) self))
      (set `self.InventoryWidget` _returnvalue_3)
      (bind _asthird_person_character (cast `/Game/MyContent/Blueprints/ThirdPersonCharacter/ThirdPersonCharacter` (`GameplayStatics.GetPlayerCharacter` 0)))
      (bind _returnvalue_4 (`CanvasPanel.AddChildToCanvas` (`/Game/MyContent/Blueprints/Inventory/Widgets/WB_HUD.HUDCanvas` (`/Game/MyContent/Blueprints/ThirdPersonCharacter/ThirdPersonCharacter.VP_HUD` _asthird_person_character)) _inventorywidget))
      (`CanvasPanelSlot.SetAutoSize` _returnvalue_4 true)
      (`CanvasPanelSlot.SetAlignment` _returnvalue_4 (1.2 0.5))
      (`CanvasPanelSlot.SetAnchors` _returnvalue_4 (make `Anchors` (0.5 0.5) (0.5 0.5)))
      (`CanvasPanelSlot.SetPosition` _returnvalue_4 (`self.Position`))
      (set `PlayerController.bShowMouseCursor` true _returnvalue_2)
      (`WidgetBlueprintLibrary.SetInputMode_GameAndUIEx` _returnvalue_2 _inventorywidget))))