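; Enemy Blueprint that loses health when hit by bullets, damages other actors that overlap it, and shows a health widget.
; Bullets, detected by an object-name substring match, reduce VidaEnemigo, and the enemy is destroyed when a second subtraction of the damage gives a negative value.
; Other overlaps start a delayed loop sending TakeDamageMessage until any overlap ends.
; The Vida_Enemigos widget receives the enemy as Owner and turns toward the player each tick.
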(event `self.ReceiveActorBeginOverlap`
  (params (OtherActor :type "Actor Object Reference"))
  (bind _returnvalue (- (`self.Vida_Enemigo`) 20.0))
  (if (`KismetStringLibrary.Contains` (`KismetSystemLibrary.GetObjectName` OtherActor) "BP_Bullet")
    (set `self.Vida_Enemigo` _returnvalue)
    (if (< _returnvalue 0.0)
      (`self.K2_DestroyActor`))
    (else
      (set `self.bool` true)
      (message `/Game/MyContent/Blueprints/Interfaces/BPI_Damageable.Take Damage` OtherActor 5.0 :!label _label)
      (`KismetSystemLibrary.Delay` 0.5)
      (if (stale `self.ReceiveActorEndOverlap` _output_get)
        (goto _label)))))

(event `self.ReceiveActorEndOverlap`
  (params (OtherActor :type "Actor Object Reference"))
  (bind _output_get (set `self.bool` false)))

(event `self.ReceiveTick`
  (params (DeltaSeconds :type "Float (single-precision)"))
  (bind _widget (`self.Widget`))
  (`SceneComponent.K2_SetWorldRotation` _widget (`KismetMathLibrary.FindLookAtRotation` (`SceneComponent.K2_GetComponentLocation` _widget) (`self.K2_GetActorLocation` (`GameplayStatics.GetPlayerCharacter` 0))) false false))

(event `self.ReceiveBeginPlay`
  ;[1 1 1] Widget
  (bind _asvida_enemigos (cast `/Game/MyContent/Blueprints/Widgets/Vida_Enemigos` (`WidgetComponent.GetUserWidgetObject` (`self.Widget`))))
  (set `/Game/MyContent/Blueprints/Widgets/Vida_Enemigos.owner` self _asvida_enemigos))

(fn `UserConstructionScript`)