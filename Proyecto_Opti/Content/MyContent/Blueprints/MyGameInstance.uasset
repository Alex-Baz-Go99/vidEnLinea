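; Game instance Blueprint that saves and loads player progress: game points and the unlock state of two skins.
; SaveGame copies these values from the ThirdPersonCharacter pawn into a new BP_SaveGame object and writes the Dataplayer slot.
; LoadGame checks that the slot exists, then copies the values back onto the pawn; both events print confirmation messages.
; Inventory and player transform nodes are present but unconnected, so neither is persisted.
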(event `SaveGame`
  (bind _asthird_person_character (cast `/Game/MyContent/Blueprints/ThirdPersonCharacter/ThirdPersonCharacter` (`GameplayStatics.GetPlayerPawn` 0) :!pure true))
  (bind _returnvalue (`GameplayStatics.CreateSaveGameObject` "/Game/MyContent/Blueprints/BP_SaveGame.BP_SaveGame_C"))
  (set `/Game/MyContent/Blueprints/BP_SaveGame.GamePoints` (`/Game/MyContent/Blueprints/ThirdPersonCharacter/ThirdPersonCharacter.GamePoints` _asthird_person_character) _returnvalue)
  (set `/Game/MyContent/Blueprints/BP_SaveGame.skin1_desbloqueada` (`/Game/MyContent/Blueprints/ThirdPersonCharacter/ThirdPersonCharacter.skin1_desbloqueda` _asthird_person_character) _returnvalue)
  (set `/Game/MyContent/Blueprints/BP_SaveGame.skin2_desbloqueada` (`/Game/MyContent/Blueprints/ThirdPersonCharacter/ThirdPersonCharacter.skin2_desbloqueda` _asthird_person_character) _returnvalue)
  (`GameplayStatics.SaveGameToSlot` null (`self.Dataplayer`))
  (`KismetSystemLibrary.PrintString` "Partida Guardada"))

(event `LoadGame`
  (bind _returnvalue (`GameplayStatics.DoesSaveGameExist` (`self.Dataplayer`)))
  (if _returnvalue
    (bind _returnvalue_2 (`GameplayStatics.LoadGameFromSlot` (`self.Dataplayer`)))
    (bind _asbp_save_game (cast `/Game/MyContent/Blueprints/BP_SaveGame` _returnvalue_2))
    (bind _asthird_person_character (cast `/Game/MyContent/Blueprints/ThirdPersonCharacter/ThirdPersonCharacter` (`GameplayStatics.GetPlayerPawn` 0)))
    (set `/Game/MyContent/Blueprints/ThirdPersonCharacter/ThirdPersonCharacter.GamePoints` (`/Game/MyContent/Blueprints/BP_SaveGame.GamePoints` _asbp_save_game) _asthird_person_character)
    (set `/Game/MyContent/Blueprints/ThirdPersonCharacter/ThirdPersonCharacter.skin1_desbloqueda` (`/Game/MyContent/Blueprints/BP_SaveGame.skin1_desbloqueada` _asbp_save_game) _asthird_person_character)
    (set `/Game/MyContent/Blueprints/ThirdPersonCharacter/ThirdPersonCharacter.skin2_desbloqueda` (`/Game/MyContent/Blueprints/BP_SaveGame.skin2_desbloqueada` _asbp_save_game) _asthird_person_character)
    (`KismetSystemLibrary.PrintString` "Partida Cargada")))