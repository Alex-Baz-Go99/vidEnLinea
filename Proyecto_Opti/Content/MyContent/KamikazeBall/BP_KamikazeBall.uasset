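; Kamikaze ball enemy character that takes damage from player projectiles and explodes when its life runs out.
; Collision overlaps match actor names to set bullet or plasma damage; the death check subtracts damage again after applying it.
; Death sets the ReachedPlayer blackboard key, skipping if already set, then spawns explosion effects and destroys the actor.
; BeginPlay sets walk speed and links the life bar widget, which Tick yaws toward the player.
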(event `self.CollisionSphere.OnComponentBeginOverlap`
  (params (OverlappedComponent :type "PrimitiveComponent Object Reference") (OtherActor :type "Actor Object Reference") (OtherComp :type "PrimitiveComponent Object Reference") (OtherBodyIndex :type Integer) (bFromSweep :type Boolean) (SweepResult :type "HitResult Structure (by ref)"))
  (bind _returnvalue (`KismetSystemLibrary.GetObjectName` OtherActor))
  (bind _returnvalue_2 (`AIBlueprintHelperLibrary.GetBlackboard` null))
  (bind _reachedplayer (`self.ReachedPlayer`))
  (bind _returnvalue_3 (- (`self.KamikazeLife`) (`self.BulletDamage`)))
  ;[1 1 1] Receive bullet damage
  (if (`KismetStringLibrary.Contains` _returnvalue "BP_Bullet")
    (set `self.BulletDamage` 20.0)
    (set `self.KamikazeLife` _returnvalue_3 :!label _label)
    (if (< _returnvalue_3 0.0)
      (if (not (`BlackboardComponent.GetValueAsBool` _returnvalue_2 _reachedplayer))
        (`BlackboardComponent.SetValueAsBool` _returnvalue_2 _reachedplayer true)
        (`GameplayStatics.SpawnEmitterAtLocation` "/Game/MyContent/Particulas/Explosion_Particles.Explosion_Particles" (`self.K2_GetActorLocation`) (struct) (0.5 0.5 0.5))
        (`GameplayStatics.PlaySound2D` "/Game/MyContent/Sounds/Explosion.Explosion" 0.1 1.0 0.0 null null)
        (`self.K2_DestroyActor`)))
    (elif (`KismetStringLibrary.Contains` _returnvalue "BP_Plasma")
      (set `self.BulletDamage` 50.0)
      (goto _label))))

(event `self.ReceiveBeginPlay`
  ;[1 1 1] Health bar
  (set `CharacterMovementComponent.MaxWalkSpeed` 250.0 (`self.CharacterMovement`))
  (bind _askamikaze_life_bar (cast `/Game/MyContent/KamikazeBall/Kamikaze_LifeBar` (`WidgetComponent.GetUserWidgetObject` (`self.Kamikaze LifeBar`))))
  (set `/Game/MyContent/KamikazeBall/Kamikaze_LifeBar.BP Kamikaze Ball` self _askamikaze_life_bar))

(event `self.ReceiveTick`
  (params (DeltaSeconds :type "Float (single-precision)"))
  (bind _kamikaze_lifebar (`self.Kamikaze LifeBar`))
  ;[1 1 1] Widget Rotation
  (`SceneComponent.K2_SetWorldRotation` _kamikaze_lifebar (`KismetMathLibrary.MakeRotator` 0.0 0.0 (.yaw (`KismetMathLibrary.FindLookAtRotation` (`SceneComponent.K2_GetComponentLocation` _kamikaze_lifebar) (`self.K2_GetActorLocation` (`GameplayStatics.GetPlayerCharacter` 0))))) false false))

(fn `UserConstructionScript`)