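; Sofa actor that swaps to a destructible version when the player touches it, then removes itself.
; On BeginPlay a timeline drives StaticMesh vertically, adding its track value to the current relative Z each update.
; A Box overlap with an actor whose display name contains "Third" teleports StaticMesh1 downward and the Destructible to the relative origin, then destroys the actor after a short delay.
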(event `self.ReceiveBeginPlay`
  (bind _staticmesh (`self.StaticMesh`))
  (bind (_direction _newtrack_0) (`Timeline|Timeline_0`)
    (:`Update`
      (`SceneComponent.K2_SetRelativeLocation` _staticmesh (+ (`KismetMathLibrary.MakeVector` 0.0 0.0 _newtrack_0) (`SceneComponent.RelativeLocation` _staticmesh)) false false))))

(event `self.Box.OnComponentBeginOverlap`
  (params (OverlappedComponent :type "PrimitiveComponent Object Reference") (OtherActor :type "Actor Object Reference") (OtherComp :type "PrimitiveComponent Object Reference") (OtherBodyIndex :type Integer) (bFromSweep :type Boolean) (SweepResult :type "HitResult Structure (by ref)"))
  (if (`KismetStringLibrary.Contains` (`KismetSystemLibrary.GetDisplayName` OtherActor) "Third")
    (`SceneComponent.K2_SetRelativeLocation` (`self.StaticMesh1`) (0.0 0.0 -300.0) false true)
    (`SceneComponent.K2_SetRelativeLocation` (`self.Destructible`) (0.0 0.0 0.0) false true)
    (`KismetSystemLibrary.Delay` 3.0)
    (`self.K2_DestroyActor`)))

(fn `UserConstructionScript`)