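; Team flag base for a capture-the-flag mode, registering itself in Steam_Game_Instance by owning team on BeginPlay.
; A construction-sized sphere detects characters: opponents pick up the flag, while teammates carrying one score and reset it.
; Pickup and reset call paired Server and Client events to update flag state.
; Scoring uses Multicast on the server or Server plus Client otherwise, incrementing TeamPoints and calling CheckPoints on player pawn 0.
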(event `Client_Reset_Flag`
  (params (Player :type "/Game/MyContent/Blueprints/ThirdPersonCharacter/ThirdPersonCharacter Object Reference"))
  ;[1 1 1] Reset flag
  (set `/Game/Blueprints/BP_FlagBase.HasFlag` true (`/Game/MyContent/Blueprints/ThirdPersonCharacter/ThirdPersonCharacter.EnemyFlagBase` Player))
  (set `/Game/MyContent/Blueprints/ThirdPersonCharacter/ThirdPersonCharacter.IsCarryingFlag` false Player))

(event `Server_Reset_Flag`
  (params (Player :type "/Game/MyContent/Blueprints/ThirdPersonCharacter/ThirdPersonCharacter Object Reference"))
  ;[1 1 1] Reset flag
  (set `/Game/Blueprints/BP_FlagBase.HasFlag` true (`/Game/MyContent/Blueprints/ThirdPersonCharacter/ThirdPersonCharacter.EnemyFlagBase` Player))
  (set `/Game/MyContent/Blueprints/ThirdPersonCharacter/ThirdPersonCharacter.IsCarryingFlag` false Player))

(event `Client_Add_Point`
  (params (FlagBase :type "/Game/Blueprints/BP_FlagBase Object Reference"))
  ;[1 1 1] Add Point
  (bind _output_get (set `self.TeamPoints` (+ (`/Game/Blueprints/BP_FlagBase.TeamPoints` FlagBase) 1)))
  (bind _asthird_person_character (cast `/Game/MyContent/Blueprints/ThirdPersonCharacter/ThirdPersonCharacter` (`GameplayStatics.GetPlayerPawn` 0)))
  (`/Game/MyContent/Blueprints/ThirdPersonCharacter/ThirdPersonCharacter.Check Points` _asthird_person_character))

(event `Server_Add_Point`
  (params (FlagBase :type "/Game/Blueprints/BP_FlagBase Object Reference"))
  ;[1 1 1] Add Point
  (bind _output_get (set `self.TeamPoints` (+ (`/Game/Blueprints/BP_FlagBase.TeamPoints` FlagBase) 1)))
  (bind _asthird_person_character (cast `/Game/MyContent/Blueprints/ThirdPersonCharacter/ThirdPersonCharacter` (`GameplayStatics.GetPlayerPawn` 0)))
  (`/Game/MyContent/Blueprints/ThirdPersonCharacter/ThirdPersonCharacter.Check Points` _asthird_person_character))

(event `Multicast_Add_Point`
  (params (FlagBase :type "/Game/Blueprints/BP_FlagBase Object Reference"))
  ;[1 1 1] Add Point
  (bind _output_get (set `self.TeamPoints` (+ (`/Game/Blueprints/BP_FlagBase.TeamPoints` FlagBase) 1)))
  (bind _asthird_person_character (cast `/Game/MyContent/Blueprints/ThirdPersonCharacter/ThirdPersonCharacter` (`GameplayStatics.GetPlayerPawn` 0)))
  (`/Game/MyContent/Blueprints/ThirdPersonCharacter/ThirdPersonCharacter.Check Points` _asthird_person_character))

(event `self.ReceiveBeginPlay`
  (bind _assteam_game_instance (cast `/Game/Steam_Session/Steam_Game_Instance` (`GameplayStatics.GetGameInstance`)))
  (if (== 1 (`self.OwnerTeam`))
    (set `/Game/Steam_Session/Steam_Game_Instance.Flag_Base_Team_1` self _assteam_game_instance)
    (else
      (set `/Game/Steam_Session/Steam_Game_Instance.Flag_Base_Team_2` self _assteam_game_instance))))

(event `Client_Player_Pickup_Flag`
  (params (Player :type "/Game/MyContent/Blueprints/ThirdPersonCharacter/ThirdPersonCharacter Object Reference"))
  ;[1 1 1] Pick up flag
  (set `/Game/Blueprints/BP_FlagBase.HasFlag` false (`/Game/MyContent/Blueprints/ThirdPersonCharacter/ThirdPersonCharacter.EnemyFlagBase` Player))
  (set `/Game/MyContent/Blueprints/ThirdPersonCharacter/ThirdPersonCharacter.IsCarryingFlag` true Player))

(event `Server_Player_Pickup_Flag`
  (params (Player :type "/Game/MyContent/Blueprints/ThirdPersonCharacter/ThirdPersonCharacter Object Reference"))
  ;[1 1 1] Pick up flag
  (set `/Game/Blueprints/BP_FlagBase.HasFlag` false (`/Game/MyContent/Blueprints/ThirdPersonCharacter/ThirdPersonCharacter.EnemyFlagBase` Player))
  (set `/Game/MyContent/Blueprints/ThirdPersonCharacter/ThirdPersonCharacter.IsCarryingFlag` true Player))

(event `self.Radious.OnComponentBeginOverlap`
  (params (OverlappedComponent :type "PrimitiveComponent Object Reference") (OtherActor :type "Actor Object Reference") (OtherComp :type "PrimitiveComponent Object Reference") (OtherBodyIndex :type Integer) (bFromSweep :type Boolean) (SweepResult :type "HitResult Structure (by ref)"))
  (bind _asthird_person_character (cast `/Game/MyContent/Blueprints/ThirdPersonCharacter/ThirdPersonCharacter` OtherActor))
  (bind _team (`/Game/MyContent/Blueprints/ThirdPersonCharacter/ThirdPersonCharacter.Team` _asthird_person_character))
  (`KismetSystemLibrary.PrintString` (`KismetStringLibrary.Conv_IntToString` _team))
  (if (== _team (`self.OwnerTeam`))
    (if (`/Game/MyContent/Blueprints/ThirdPersonCharacter/ThirdPersonCharacter.IsCarryingFlag` _asthird_person_character)
      (if (`KismetSystemLibrary.IsServer`)
        (bind _myflagbase (`/Game/MyContent/Blueprints/ThirdPersonCharacter/ThirdPersonCharacter.MyFlagBase` _asthird_person_character))
        (`self.Multicast_Add_Point` _myflagbase _myflagbase)
        (else
          (`self.Server_Add_Point` _myflagbase _myflagbase)
          (`self.Client_Add_Point` _myflagbase _myflagbase)))
      (`self.Server_Reset_Flag` _asthird_person_character)
      (`self.Client_Reset_Flag` _asthird_person_character))
    (else
      (`self.Server_Player_Pickup_Flag` _asthird_person_character)
      (`self.Client_Player_Pickup_Flag` _asthird_person_character))))

(fn `OnRep_HasFlag`)

(fn `OnRep_OwnerTeam`)

(fn `OnRep_TeamPoints`)

(fn `UserConstructionScript`
  (`SphereComponent.SetSphereRadius` (`self.Radious`) (`self.RadiousValue`) true))