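; AI mutant enemy that melees the player, takes projectile damage and awards score on death.
; MutantAttack plays a montage whose notify fires a left-hand sphere trace, damaging the player matched by display name.
; Bullet and plasma overlaps, told apart by object name, drain life until death sets a Blackboard flag, plays a montage, destroys the actor and adds a point.
; A life-bar widget references the enemy and yaws toward the player each tick.
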(event `/Game/Biomech_Mutant/ADAI/CombatInterface.MutantAttack`
  (bind _returnvalue (`SceneComponent.GetSocketLocation` (`self.Mesh`) "hand_lSocket"))
  (`|PlayMontage` (`self.Mesh`) "/Game/Biomech_Mutant/ADAI/BP_ADAIEnemy_Attack.BP_ADAIEnemy_Attack"
    (:`then`
      (`GameplayStatics.PlaySound2D` "/Game/MyContent/Sounds/AtaqueAIEnemy.AtaqueAIEnemy" 1.0 1.0 0.0 null null))
    (:`OnNotifyBegin`
      (bind _outhit (`KismetSystemLibrary.SphereTraceSingle` _returnvalue (+ _returnvalue (* (`KismetMathLibrary.GetForwardVector` (`self.K2_GetActorRotation`)) (`self.RangeOfAttack`))) (`self.SizeofSphere`) "TraceTypeQuery2"))
      (if (`KismetStringLibrary.EqualEqual_StrStr` (`KismetSystemLibrary.GetDisplayName` (`.HitActor` (`GameplayStatics.BreakHitResult` _outhit))) "ThirdPersonCharacter")
        (message `/Game/MyContent/Blueprints/Interfaces/BPI_Damageable.Take Damage` (`.HitActor` (`GameplayStatics.BreakHitResult` _outhit)) 5.0)))))

(event `self.ReceiveActorBeginOverlap`
  (params (OtherActor :type "Actor Object Reference"))
  (bind _returnvalue (`KismetSystemLibrary.GetObjectName` OtherActor))
  (bind _returnvalue_2 (`AIBlueprintHelperLibrary.GetBlackboard` null))
  (bind _mutantdead (`self.MutantDead`))
  (bind _returnvalue_3 (- (`self.ADAI_Life`) (`self.BulletDamage`)))
  ;[1 1 1] Receive bullet damage
  (if (`KismetStringLibrary.Contains` _returnvalue "BP_Bullet")
    (set `self.BulletDamage` 20.0)
    (set `self.ADAI_Life` _returnvalue_3 :!label _label)
    (if (< _returnvalue_3 0.0)
      (if (not (`BlackboardComponent.GetValueAsBool` _returnvalue_2 _mutantdead))
        (`BlackboardComponent.SetValueAsBool` _returnvalue_2 _mutantdead true)
        (`|PlayMontage` (`self.Mesh`) "/Game/MyContent/Blueprints/Enemy/BP_AIEnemy_Die.BP_AIEnemy_Die" 1.0 1.3
          (:`then`
            (`KismetSystemLibrary.Delay` 1.5)
            (`self.K2_DestroyActor`)
            (bind _asthird_person_game_mode (cast `/Game/ThirdPersonBP/Blueprints/ThirdPersonGameMode` (`GameplayStatics.GetGameMode`)))
            (`/Game/ThirdPersonBP/Blueprints/ThirdPersonGameMode.AddScorePoints` _asthird_person_game_mode 1)))))
    (elif (`KismetStringLibrary.Contains` _returnvalue "BP_Plasma")
      (set `self.BulletDamage` 50.0)
      (goto _label))))

(event `self.ReceiveBeginPlay`
  ;[1 1 1] Health bar
  (bind _asadai_life_bar (cast `/Game/Biomech_Mutant/ADAI/ADAI_LifeBar` (`WidgetComponent.GetUserWidgetObject` (`self.ADAI LifeBar`))))
  (set `/Game/Biomech_Mutant/ADAI/ADAI_LifeBar.BP ADAI Enemy reference` self _asadai_life_bar))

(event `self.ReceiveTick`
  (params (DeltaSeconds :type "Float (single-precision)"))
  (bind _adai_lifebar (`self.ADAI LifeBar`))
  ;[1 1 1] Widget Rotation
  (`SceneComponent.K2_SetWorldRotation` _adai_lifebar (`KismetMathLibrary.MakeRotator` 0.0 0.0 (.yaw (`KismetMathLibrary.FindLookAtRotation` (`SceneComponent.K2_GetComponentLocation` _adai_lifebar) (`self.K2_GetActorLocation` (`GameplayStatics.GetPlayerCharacter` 0))))) false false))

(fn `UserConstructionScript`)