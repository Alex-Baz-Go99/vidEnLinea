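; Enemy AI mutant that chases the player, plays melee attacks and awards score on death.
; Pawn sensing or the first hit starts AIMoveTo; reaching the player triggers a rate-limited attack montage and sound.
; Overlaps identify bullets or plasma by object name to subtract health, while other actors take damage every second until overlap ends.
; A health-bar widget references the enemy and yaw-rotates toward the player each tick.
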(event `self.ReceiveActorBeginOverlap`
  (params (OtherActor :type "Actor Object Reference"))
  (bind _returnvalue (`KismetSystemLibrary.GetObjectName` OtherActor))
  (bind _returnvalue_2 (- (`self.AI Enemy life`) (`self.Damage`)))
  ;[1 1 1] Receive/make damage
  (if (`KismetStringLibrary.Contains` _returnvalue "BP_Bullet")
    (`KismetSystemLibrary.PrintString` "poco")
    (set `self.Damage` 10.0)
    (if (not (`self.already_following`)) :!label _label
      (set `self.already_following` true)
      (set `self.Hit_Once` true))
    (set `self.AI Enemy life` _returnvalue_2)
    (if (< _returnvalue_2 0.0)
      (if (not (`self.Dead`))
        (set `self.Dead` true)
        (`|PlayMontage` (`self.Mesh`) "/Game/MyContent/Blueprints/Enemy/BP_AIEnemy_Die.BP_AIEnemy_Die" 1.0 1.3
          (:`then`
            (`KismetSystemLibrary.Delay` 1.5)
            (`self.K2_DestroyActor`)
            (bind _asthird_person_game_mode (cast `/Game/ThirdPersonBP/Blueprints/ThirdPersonGameMode` (`GameplayStatics.GetGameMode`)))
            (`/Game/ThirdPersonBP/Blueprints/ThirdPersonGameMode.AddScorePoints` _asthird_person_game_mode (`self.Add Score Point`))))))
    (elif (`KismetStringLibrary.Contains` _returnvalue "BP_Plasma")
      (`KismetSystemLibrary.PrintString` "mucho")
      (set `self.Damage` 25.0)
      (goto _label)
      (elif (not (`self.Dead`))
        (set `self.AI bool` true)
        (message `/Game/MyContent/Blueprints/Interfaces/BPI_Damageable.Take Damage` OtherActor 5.0 :!label _label_2)
        (`KismetSystemLibrary.Delay` 1.0)
        (if (stale `self.ReceiveActorEndOverlap` _output_get)
          (goto _label_2))))))

(event `self.ReceiveActorEndOverlap`
  (params (OtherActor :type "Actor Object Reference"))
  ;[1 1 1] Receive/make damage
  (bind _output_get (set `self.AI bool` false)))

(event `self.ReceiveTick`
  (params (DeltaSeconds :type "Float (single-precision)"))
  (bind _ai_life_widget (`self.AI Life Widget`))
  ;[1 1 1] Widget Rotation
  (`|ExecutionSequence`
    (:`then_0`
      (`SceneComponent.K2_SetWorldRotation` _ai_life_widget (`KismetMathLibrary.MakeRotator` 0.0 0.0 (.yaw (`KismetMathLibrary.FindLookAtRotation` (`SceneComponent.K2_GetComponentLocation` _ai_life_widget) (`self.K2_GetActorLocation` (`GameplayStatics.GetPlayerCharacter` 0))))) false false))
    (:`then_1`
      (if (`self.Hit_Once`)
        (set `self.Hit_Once` false)
        (`|AIMoveTo` self (0.0 0.0 0.0) (`GameplayStatics.GetPlayerPawn` 0) 12.0 :!label _label_3
          (:`OnSuccess`
            (if (`self.Dead`)
              _
              (elif (`self.Can Attack`)
                (set `self.Can Attack` false)
                (`|PlayMontage` (`self.Mesh`) "/Game/MyContent/Blueprints/Enemy/BP_AIEnemy_Attack.BP_AIEnemy_Attack"
                  (:`then`
                    (`GameplayStatics.PlaySound2D` "/Game/MyContent/Sounds/AtaqueAIEnemy.AtaqueAIEnemy" 1.0 1.0 0.0 null null)
                    (`KismetSystemLibrary.Delay` (`self.Attack Rate`))
                    (set `self.Can Attack` true)))))))))))

(event `self.ReceiveBeginPlay`
  ;[1 1 1] Health bar
  (bind _asaienemy_life (cast `/Game/MyContent/Blueprints/Widgets/AIEnemy_Life` (`WidgetComponent.GetUserWidgetObject` (`self.AI Life Widget`))))
  (set `/Game/MyContent/Blueprints/Widgets/AIEnemy_Life.BP AI Enemy reference` self _asaienemy_life))

(event `self.PawnSensing.OnSeePawn`
  (params (Pawn :type "Pawn Object Reference"))
  (goto _label_3))

(fn `UserConstructionScript`)